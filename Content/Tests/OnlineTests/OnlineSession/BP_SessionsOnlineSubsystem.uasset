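; Test helper Blueprint for online session tests that relays session operation results to a functional test.
; It handles completion events for creating, destroying, starting, ending and finding sessions.
; Each event passes its success flag or found sessions unchanged to the same-named function on the FunctionalTest reference, with no logic of its own.
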(event EventOnDestroySessionCompleted
  (params (wasSuccessful :type Boolean))
  (Class|MSFunctionalTest|OnDestroySessionCompleted (Utilities|ResolveSoftReference (Variables|Default|GetFunctionalTest)) wasSuccessful))

(event EventOnFindSessionsCompleted
  (params (sessions :type Array%20of%20Strings))
  (Class|MSFunctionalTest|OnFindSessionsCompleted (Utilities|ResolveSoftReference (Variables|Default|GetFunctionalTest)) sessions))

(event EventOnCreateSessionCompleted
  (params (wasSuccessful :type Boolean))
  (Class|MSFunctionalTest|OnCreateSessionCompleted (Utilities|ResolveSoftReference (Variables|Default|GetFunctionalTest)) wasSuccessful))

(event EventOnStartSessionCompleted
  (params (wasSuccessful :type Boolean))
  (Class|MSFunctionalTest|OnStartSessionCompleted (Utilities|ResolveSoftReference (Variables|Default|GetFunctionalTest)) wasSuccessful))

(event EventOnEndSessionCompleted
  (params (wasSuccessful :type Boolean))
  (Class|MSFunctionalTest|OnEndSessionCompleted (Utilities|ResolveSoftReference (Variables|Default|GetFunctionalTest)) wasSuccessful))

(fn ConstructionScript)