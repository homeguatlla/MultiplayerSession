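; Functional test that verifies an online session can be created and then destroyed through the OnlineSubsystem.
; StartTest creates a session, and its create-and-start completion event triggers the destroy call.
; The test succeeds when destruction completes successfully and fails with an error message if either step reports failure.
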(event EventOnCreateandStartSessionCompleted
  (params (bWasSuccessful :type Boolean))
  (if bWasSuccessful
    (Class|BPOnlineSubsystem|DestroySession (Variables|Default|GetOnlineSubsystem))
    (else
      (Class|FunctionalTest|FinishTest "Failed" "Error creating Session"))))

(event EventStartTest
  (Class|BPOnlineSubsystem|CreateSession (Variables|Default|GetOnlineSubsystem)))

(event EventOnDestroySessionCompleted
  (params (bWasSuccessful :type Boolean))
  (if bWasSuccessful
    (Class|FunctionalTest|FinishTest "Succeeded" "Session created and destroyed")
    (else
      (Class|FunctionalTest|FinishTest "Failed" "Error destroying the already created session"))))

(fn ConstructionScript)