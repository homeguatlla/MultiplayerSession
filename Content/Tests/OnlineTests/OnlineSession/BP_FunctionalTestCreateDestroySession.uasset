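; Functional test that checks the online subsystem can create and then destroy a session.
; StartTest requests session creation; a successful completion event triggers destruction, whose completion event marks the test succeeded or failed.
; A creation failure fails the test immediately.
; Every outcome quits the game after finishing the test.
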(event EventStartTest
  (Class|BPSessionsOnlineSubsystem|CreateSession (Variables|Default|GetOnlineSubsystem)))

(event EventOnDestroySessionCompleted
  (params (wasSuccessful :type Boolean))
  (if wasSuccessful
    (Class|FunctionalTest|FinishTest "Succeeded" "Session created and destroyed")
    (else
      (Class|FunctionalTest|FinishTest "Failed" "Session created but not destroyed")))
  (Game|QuitGame 0 "Quit" false))

(event EventOnCreateSessionCompleted
  (params (wasSuccessful :type Boolean))
  (if wasSuccessful
    (Class|BPSessionsOnlineSubsystem|DestroySession (Variables|Default|GetOnlineSubsystem))
    (else
      (Class|FunctionalTest|FinishTest "Failed" "Error creating Session")
      (Game|QuitGame 0 "Quit" false))))

(fn ConstructionScript)