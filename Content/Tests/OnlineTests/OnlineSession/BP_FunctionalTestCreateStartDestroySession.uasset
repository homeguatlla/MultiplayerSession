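; Functional test that checks online session creation, start and destruction through the OnlineSubsystem.
; StartTest creates the session, and a successful create-and-start callback triggers DestroySession.
; The test succeeds only when destruction completes, reports a distinct message for each failed stage, and quits the game on every outcome.
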(event EventOnCreateandStartSessionCompleted
  (params (bWasSuccessful :type Boolean))
  (if bWasSuccessful
    (Class|BPOnlineSubsystem|DestroySession (Variables|Default|GetOnlineSubsystem))
    (else
      (Class|FunctionalTest|FinishTest "Failed" "Error creating Session")
      (Game|QuitGame 0 "Quit" false))))

(event EventStartTest
  (Class|BPOnlineSubsystem|CreateSession (Variables|Default|GetOnlineSubsystem)))

(event EventOnDestroySessionCompleted
  (params (bWasSuccessful :type Boolean))
  (if bWasSuccessful
    (Class|FunctionalTest|FinishTest "Succeeded" "Session created and destroyed")
    (else
      (Class|FunctionalTest|FinishTest "Failed" "Session created but not destroyed")))
  (Game|QuitGame 0 "Quit" false))

(fn ConstructionScript)