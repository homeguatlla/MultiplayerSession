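; Functional test that verifies the online session lifecycle: create, start, end and destroy.
; StartTest creates a session, and each completion event triggers the next OnlineSubsystem step on success.
; Any failure fails the test with a stage-specific message, while a successful destroy passes it.
; Every outcome then quits the game.
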(event EventOnCreateSessionCompleted
  (params (wasSuccessful :type Boolean))
  (if wasSuccessful
    (Class|BPOnlineSubsystem|StartSession (Variables|Default|GetOnlineSubsystem))
    (else
      (Class|FunctionalTest|FinishTest "Failed" "Error creating Session")
      (Game|QuitGame 0 "Quit" false))))

(event EventStartTest
  (Class|BPOnlineSubsystem|CreateSession (Variables|Default|GetOnlineSubsystem)))

(event EventOnDestroySessionCompleted
  (params (wasSuccessful :type Boolean))
  (if wasSuccessful
    (Class|FunctionalTest|FinishTest "Succeeded")
    (else
      (Class|FunctionalTest|FinishTest "Failed" "Session created but not destroyed")))
  (Game|QuitGame 0 "Quit" false))

(event EventOnStartSessionCompleted
  (params (wasSuccessful :type Boolean))
  (if wasSuccessful
    (Class|BPOnlineSubsystem|EndSession (Variables|Default|GetOnlineSubsystem))
    (else
      (Class|FunctionalTest|FinishTest "Failed" "Error starting session")
      (Game|QuitGame 0 "Quit" false))))

(event EventOnEndSessionCompleted
  (params (wasSuccessful :type Boolean))
  (if wasSuccessful
    (Class|BPOnlineSubsystem|DestroySession (Variables|Default|GetOnlineSubsystem))
    (else
      (Class|FunctionalTest|FinishTest "Failed" "Error ending session")
      (Game|QuitGame 0 "Quit" false))))

(fn ConstructionScript)